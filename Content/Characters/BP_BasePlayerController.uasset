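; BP_BasePlayerController is a player controller Blueprint that routes player input and creates the inventory UI.
; On BeginPlay it creates a UI_Inventory widget and stores it as InventoryWidget0, a step noted to move to C++.
; Input actions forward left click press and release, camera zoom in and out, and the inventory key to functions whose bodies are not defined in this graph.
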(event EventBeginPlay
  ;[1 1 1] Move this to c++
  (bind _returnvalue (UserInterface|CreateWidget "/Game/UI/UI_Inventory.UI_Inventory_C"))
  (Variables|Default|SetInventoryWidget_0 _returnvalue))

(event EventTick
  (params (DeltaSeconds :type Float%20%28single-precision%29)))

(event Input|ActionEvents|InputActionLeftClick
  (params (Key :type Key%20Structure))
  (:Pressed
    (Class|BasePlayerController|OnLeftClick))
  (:Released
    (Class|BasePlayerController|OnLeftClickRelease)))

(event Input|ActionEvents|InputActionZoomIn
  (params (Key :type Key%20Structure))
  (:Pressed
    (Class|BasePlayerController|ChangeCameraZoom true)))

(event Input|ActionEvents|InputActionZoomOut
  (params (Key :type Key%20Structure))
  (:Pressed
    (Class|BasePlayerController|ChangeCameraZoom false)))

(event Input|ActionEvents|InputActionInventory
  (params (Key :type Key%20Structure))
  (:Pressed
    (Class|BasePlayerController|ShowInventory)))

(fn ConstructionScript)