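; Active skill Blueprint for a basic melee attack against a target actor.
; Use validates the target and user, turns the user to face the target, then deals fixed physical damage credited to the user and its controller.
; It returns success after a debug print, or false if either actor is invalid.
; Range is set at BeginPlay, but it and a distance node are unused, so no range check occurs.
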(event EventBeginPlay
  (Variables|Default|SetRange 1e+02))

(event EventTick
  (params (DeltaSeconds :type Float%20%28single-precision%29)))

(fn Use
  (params (User :type Base%20Entity%20Object%20Reference) (Target :type Base%20Entity%20Object%20Reference) (TargetLocation :type Vector :default "0, 0, 0"))
  (Utilities|IsValid Target
    (:Is%20Valid
      (Utilities|IsValid User
        (:Is%20Valid
          (Class|BaseEntity|FaceActor User Target)
          (Class|BaseEntity|DealDamageBP Target (Utilities|Struct|MakeDamageInfo (Utilities|Map|MakeMap "None" 1e+01) (Utilities|Map|MakeMap)) User (Pawn|GetController User))
          (Development|PrintString "Hello")
          (return true))
        (:Is%20Not%20Valid
          _)))
    (:Is%20Not%20Valid
      _))
  (return false))